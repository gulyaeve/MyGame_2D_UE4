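; Player-controlled 2D sprite character with four-directional movement and matching Paper2D flipbook animations.
; Two axis inputs scale MaxSpeed into movement along the actor's forward and right vectors, which Tick consumes and applies as a swept local offset.
; Each axis event also updates Direction, prioritizing up/down over left/right, and selects that direction's walk flipbook, or the last direction's idle flipbook when stationary.
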(event EventBeginPlay)

(event Collision|EventActorBeginOverlap
  (params (OtherActor :type Actor%20Object%20Reference)))

(event EventTick
  (params (DeltaSeconds :type Float%20%28single-precision%29))
  (bind _returnvalue (Class|Pawn|ConsumeMovementInputVector))
  (Transformation|AddActorLocalOffset (* _returnvalue DeltaSeconds) true false))

(event Input|AxisEvents|InputAxisAxisUP
  (params (AxisValue :type Float%20%28single-precision%29))
  (bind _output_get (Variables|Default|SetSpeedUp (* (Variables|Default|GetMaxSpeed) AxisValue)))
  (Pawn|Input|AddMovementInput (Transformation|GetActorForwardVector) _output_get false)
  (CallFunction|Animation))

(event Input|AxisEvents|InputAxisAxisRight
  (params (AxisValue :type Float%20%28single-precision%29))
  (bind _output_get (Variables|Default|SetSpeedRight (* (Variables|Default|GetMaxSpeed) AxisValue)))
  (Pawn|Input|AddMovementInput (Transformation|GetActorRightVector) _output_get false)
  (CallFunction|Animation))

(fn ConstructionScript)

(fn Animation
  (bind _speedup (Variables|Default|GetSpeedUp))
  (bind _speedright (Variables|Default|GetSpeedRight))
  (if (> _speedup 0.0)
    (Variables|Default|SetDirection "NewEnumerator0")
    (CallFunction|WalkAnimation :!label _label)
    (elif (< _speedup 0.0)
      (Variables|Default|SetDirection "NewEnumerator3")
      (goto _label)
      (elif (> _speedright 0.0)
        (Variables|Default|SetDirection "NewEnumerator2")
        (goto _label)
        (elif (< _speedright 0.0)
          (Variables|Default|SetDirection "NewEnumerator1")
          (goto _label)
          (else
            (CallFunction|IdleAnimation)))))))

(fn IdleAnimation
  (Sprite|SetFlipbook (Variables|Default|GetPaperFlipbook) (Utilities|Select :Index (Variables|Default|GetDirection) :NewEnumerator0 (Variables|IdleAnim|GetIdleUp) :NewEnumerator1 (Variables|IdleAnim|GetIdleLeft) :NewEnumerator2 (Variables|IdleAnim|GetIdleRight) :NewEnumerator3 (Variables|IdleAnim|GetIdleDown))))

(fn WalkAnimation
  (Sprite|SetFlipbook (Variables|Default|GetPaperFlipbook) (Utilities|Select :Index (Variables|Default|GetDirection) :NewEnumerator0 (Variables|WalkAnim|GetWalkUp) :NewEnumerator1 (Variables|WalkAnim|GetWalkLeft) :NewEnumerator2 (Variables|WalkAnim|GetWalkRight) :NewEnumerator3 (Variables|WalkAnim|GetWalkDown))))